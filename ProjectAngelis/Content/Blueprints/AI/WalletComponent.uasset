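; Wallet component that tracks a balance of funds, earned from defeated characters and spent when items are sold.
; On initialization it binds handlers to the character-defeated and item-sold events.
; A defeat adds the small, medium or large reward matching the character's size, while a sale subtracts the item's cost.
; Two helper functions update the balance directly, with no check against it going negative.
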(event Custom|RewardPoints
  (params (CharacerSize :type Size%20Enum%20%28by%20ref%29 :default "NewEnumerator0"))
  (switch Utilities|FlowControl|Switch|SwitchonSize CharacerSize
    (:NewEnumerator0
      (CallFunction|AddFundstoWallet (Variables|Default|GetRewardSmall)))
    (:NewEnumerator1
      (CallFunction|AddFundstoWallet (Variables|Default|GetRewardMedium)))
    (:NewEnumerator2
      (CallFunction|AddFundstoWallet (Variables|Default|GetRewardLarge)))))

(event Custom|ItemSoldEvent
  (params (ItemCost :type Integer%20%28by%20ref%29))
  (CallFunction|SubtractFundsfromWallet ItemCost))

(event EventTick
  (params (DeltaSeconds :type Float%20%28single-precision%29)))

(event EventInitializeComponent
  (EventDispatchers|BindEventtoCharacterDefeated (delegate Custom|RewardPoints))
  (EventDispatchers|BindEventtoItemSold (delegate Custom|ItemSoldEvent)))

(fn AddFundstoWallet
  (params (FundstoAdd :type Integer%20%28by%20ref%29 :default 0))
  (Variables|Default|SetCurrentFundsInWallet (+ (Variables|Default|GetCurrentFundsInWallet) FundstoAdd)))

(fn SubtractFundsfromWallet
  (params (FundsToSubtract :type Integer%20%28by%20ref%29 :default 0))
  (Variables|Default|SetCurrentFundsInWallet (- (Variables|Default|GetCurrentFundsInWallet) FundsToSubtract)))