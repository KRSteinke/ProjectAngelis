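; Inventory component that stores a character's weapons in an array, tracks the current index and attaches weapons to the owning actor.
; PickupWeapon adds and equips a weapon, or drops and replaces the current one at capacity, while GiveWeapon skips that check for AI setup or cheats.
; SwitchWeapon attaches a neighboring slot without updating the index or checking bounds.
; WeaponDrop always removes the current weapon, and its detach function is an empty stub.
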(event Custom|PickupWeapon
  (params (PickedUpWeapon :type Weapon%20Object%20Reference%20%28by%20ref%29))
  (bind _weaponinventoryarray (Variables|Default|GetWeaponInventoryArray))
  ;[1 1 1] When this event is called, a check is made to see whether character is already carrying max amount of weapons, if not the weapon is added to inventory and weapon is equiped, if character has maximum amount of weapons, the current weapon is dropped and replaced with the newly picked up weapon
  (if (== (Utilities|Array|Length (Variables|Default|GetWeaponInventoryArray)) (Variables|Default|GetMaxInventorySize))
    (CallFunction|WeaponDrop (Utilities|Array|Get(acopy) _weaponinventoryarray (Variables|Default|GetCurrentInventoryIndex)))
    (Utilities|Array|SetArrayElem _weaponinventoryarray (Variables|Default|GetCurrentInventoryIndex) PickedUpWeapon)
    (CallFunction|AttachWeapontoActor (Variables|Default|GetCurrentInventoryIndex))
    (else
      (bind _returnvalue (Utilities|Array|Add (Variables|Default|GetWeaponInventoryArray) PickedUpWeapon))
      (bind _output_get (Variables|Default|SetCurrentInventoryIndex _returnvalue))
      (CallFunction|AttachWeapontoActor _output_get))))

(event Custom|SwitchWeapon
  (params (SwitchUp :type Boolean%20%28by%20ref%29 :default false))
  ;[1 1 1] When Character Switches Weapon, current weapon is detached from character than iterates through inventory and attaches next Weapon based on parameter given
  (Class|Actor|DetachRootComponentfromParent (Utilities|Array|Get(acopy) (Variables|Default|GetWeaponInventoryArray) (Variables|Default|GetCurrentInventoryIndex)) true)
  (if SwitchUp
    (CallFunction|AttachWeapontoActor (+ (Variables|Default|GetCurrentInventoryIndex) 1))
    (else
      (CallFunction|AttachWeapontoActor (+ (Variables|Default|GetCurrentInventoryIndex) -1)))))

(event Custom|WeaponDrop
  (params (WeaponToDrop :type Weapon%20Object%20Reference%20%28by%20ref%29))
  (bind _weaponinventoryarray (Variables|Default|GetWeaponInventoryArray))
  (bind _currentinventoryindex (Variables|Default|GetCurrentInventoryIndex))
  (bind _item (Utilities|Array|Get(acopy) _weaponinventoryarray _currentinventoryindex))
  ;[1 1 1] This event unattaches a weapon from the characters inventory and removes it from character's inventory array
  (CallFunction|UnAttachWeapontoActor _item)
  (Utilities|Array|RemoveItem _weaponinventoryarray _item))

(event Custom|GiveWeapon
  (params (WeaponToGive :type Weapon%20Object%20Reference%20%28by%20ref%29))
  ;[1 1 1] This Event gives a Character s weapon and equips/attaches it, there is no check if the character is already holding max amount of weapons, primarily meant for initializing AI or for God spawn cheats for players
  (bind _returnvalue (Utilities|Array|Add (Variables|Default|GetWeaponInventoryArray) WeaponToGive))
  (bind _output_get (Variables|Default|SetCurrentInventoryIndex _returnvalue))
  (CallFunction|AttachWeapontoActor _output_get))

(event EventTick
  (params (DeltaSeconds :type Float%20%28single-precision%29)))

(event EventInitializeComponent)

(fn AttachWeapontoActor
  (params (WeaponFromInventoryIndex :type Integer%20%28by%20ref%29 :default 0))
  (Class|Actor|AttachRootComponenttoActor (Utilities|Array|Get(acopy) (Variables|Default|GetWeaponInventoryArray) WeaponFromInventoryIndex) (Components|GetOwner) "None" "SnapToTarget" true))

(fn UnAttachWeapontoActor
  (params (WeaponToUnequip :type Weapon%20Object%20Reference%20%28by%20ref%29)))

(fn GetCurrentWeapon
  (return (Utilities|Array|Get(acopy) (Variables|Default|GetWeaponInventoryArray) (Variables|Default|GetCurrentInventoryIndex))))