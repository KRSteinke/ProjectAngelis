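; VR game mode that runs wave-based zombie spawning.
; InitWave advances the wave, splits its enemy count into five-member squads plus a remainder, and starts a looping spawn timer.
; Each tick spawns a squad of AI running the zombie behavior tree at one of five randomly picked points.
; Medium and heavy per-squad counts are computed but unused in spawning; AwardPoints is empty, and automatic next-wave logic is disconnected.
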(fn ConstructionScript)

(fn FindNumMeds
  (params (NumSquads :type Integer :default 0))
  (bind _wavenumber (Variables|Default|GetWaveNumber))
  (bind _medenemies (Variables|Default|GetMedEnemies))
  (bind _item (Utilities|Array|Get(acopy) _medenemies _wavenumber))
  (Variables|SquadComp|SetMedsPerSquad (/ _item NumSquads))
  (Variables|SquadComp|SetMedSpares (Math|Integer|%(Integer) _item NumSquads)))

(fn SpawnSingleSquad
  (params (SquadSize :type Integer :default 0) (SpawnPoint :type My%20Target%20Point%20Object%20Reference))
  (for _index (range 1 SquadSize)
    (AI|SpawnAIFromClass 0 "/Game/Blueprints/AI/Zombie/ZombieBehaviorTree.ZombieBehaviorTree" (Transformation|GetActorLocation SpawnPoint) (Transformation|GetActorRotation SpawnPoint) false)))

(fn SpawnSquadfromEnemy
  (bind _lastsquadnum (Variables|Default|GetLastSquadNum))
  (Variables|SquadComp|SetMember%20Number 1)
  (if (== 0 (Variables|Default|GetNumSquads))
    (if (not (== _lastsquadnum 0))
      (Utilities|RandomSpawnPoint
        (:Output
          (CallFunction|SpawnSingleSquad _lastsquadnum (Variables|Default|GetSpawnPoint)))))
    (else
      (Utilities|RandomSpawnPoint
        (:Output
          (CallFunction|SpawnSingleSquad 5 (Variables|Default|GetSpawnPoint)))))))

(fn InitWave
  (bind _numsquads (Variables|Default|GetNumSquads))
  (bind _returnvalue (+ _numsquads 1))
  (Variables|Default|SetSquadNum 0)
  (Variables|Default|SetWaveNumber (+ (Variables|Default|GetWaveNumber) 1))
  (CallFunction|FindNumSquads)
  (if (== (Variables|Default|GetLastSquadNum) 0)
    (CallFunction|FindNumMeds _numsquads)
    (CallFunction|FindNumHeavy _numsquads)
    (else
      (CallFunction|FindNumMeds _returnvalue)
      (CallFunction|FindNumHeavy _returnvalue)))
  (Utilities|Time|SetTimerbyFunctionName self "SpawnSquadFromEnemy" 2e+01 true))

(fn FindNumSquads
  (bind _enemynum (Variables|Default|GetEnemyNum))
  (bind _wavenumber (Variables|Default|GetWaveNumber))
  (bind _item (Utilities|Array|Get(acopy) _enemynum _wavenumber))
  (Variables|Default|SetCurrentEnemies _item)
  (Variables|Default|SetNumSquads (/ _item 5))
  (Variables|Default|SetLastSquadNum (Math|Integer|%(Integer) _item 5)))

(fn FindNumHeavy
  (params (NumSquads :type Integer :default 0))
  (bind _wavenumber (Variables|Default|GetWaveNumber))
  (bind _heavyenemies (Variables|Default|GetHeavyEnemies))
  (bind _item (Utilities|Array|Get(acopy) _heavyenemies _wavenumber))
  (Variables|SquadComp|SetHeavyPerSquad (/ _item NumSquads))
  (Variables|SquadComp|SetHeavySpares (Math|Integer|%(Integer) _item NumSquads)))

(fn AwardPoints
  (params (Points :type Integer :default 0)))