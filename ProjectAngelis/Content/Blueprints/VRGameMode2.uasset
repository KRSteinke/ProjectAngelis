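; VR game mode that runs enemy waves, spawning AI squads at five spawn points.
; InitWave advances the wave, plays a countdown sound, splits the enemy count into squads of five plus remainder, and starts a looping ten-second spawn timer.
; Each tick spawns an AngelisEnemy2 squad at a random point; NumSquads never decrements and the timer never clears here.
; Medium and heavy per-squad counts are computed but unused in spawning.
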(event EventBeginPlay)

(event EventTick
  (params (DeltaSeconds :type Float%20%28single-precision%29)))

(fn ConstructionScript)

(fn SpawnEnemy
  (bind _spawnpoint1 (Variables|Default|GetSpawnPoint1))
  (AI|SpawnAIFromClass "/Game/Blueprints/AI/ProjectAngelisAI/AIGuard/AngelisEnemy2.AngelisEnemy2_C" "/Game/Blueprints/AI/ProjectAngelisAI/ProjectAngelisBT.ProjectAngelisBT" (Transformation|GetActorLocation _spawnpoint1) (Transformation|GetActorRotation _spawnpoint1) false))

(fn InitWave
  (bind _numsquads (Variables|Default|GetNumSquads))
  (bind _returnvalue (+ _numsquads 1))
  (Audio|PlaySoundatLocation "/Game/Audio/Sounds/countdown_person.countdown_person" "0, 0, 0")
  (Variables|Default|SetSquadNum 0)
  (bind _output_get (Variables|Default|SetWaveNumber (+ (Variables|Default|GetWaveNumber) 1)))
  (Variables|Default|SetCurrentEnemies (Utilities|Array|Get(acopy) (Variables|Default|GetEnemyNum) _output_get))
  (CallFunction|FindNumSquads)
  (if (== (Variables|Default|GetLastSquadNum) 0)
    (CallFunction|FindNumMeds _numsquads)
    ;[1 1 1] Find Num Heavies
    (CallFunction|FindNumHeavy _numsquads)
    (else
      ;[1 1 1] Find Num Meds
      (CallFunction|FindNumMeds _returnvalue)
      ;[1 1 1] Find Num Heavies
      (CallFunction|FindNumHeavy _returnvalue)))
  (Utilities|Time|SetTimerbyFunctionName self "SpawnSquadFromEnemy" 1e+01 true))

(fn FindNumMeds
  (params (NumSquads :type Integer :default 0))
  (bind _wavenumber (Variables|Default|GetWaveNumber))
  (bind _medenemies (Variables|Default|GetMedEnemies))
  (bind _item (Utilities|Array|Get(acopy) _medenemies _wavenumber))
  (Variables|Default|SetMedsPerSquad (/ _item NumSquads))
  (Variables|Default|SetMedSpares (Math|Integer|%(Integer) _item NumSquads)))

(fn FindNumSquads
  (bind _enemynum (Variables|Default|GetEnemyNum))
  (bind _wavenumber (Variables|Default|GetWaveNumber))
  (bind _item (Utilities|Array|Get(acopy) _enemynum _wavenumber))
  (Variables|Default|SetCurrentEnemies _item)
  (Variables|Default|SetNumSquads (/ _item 5))
  (Variables|Default|SetLastSquadNum (Math|Integer|%(Integer) _item 5)))

(fn FindNumHeavy
  (params (NumSquads :type Integer :default 0))
  (bind _wavenumber (Variables|Default|GetWaveNumber))
  (bind _heavyenemies (Variables|Default|GetHeavyEnemies))
  (bind _item (Utilities|Array|Get(acopy) _heavyenemies _wavenumber))
  (Variables|Default|SetHeavyPerSquad (/ _item NumSquads))
  (Variables|Default|SetHeavySpares (Math|Integer|%(Integer) _item NumSquads)))

(fn SpawnSquadfromEnemy
  (bind _lastsquadnum (Variables|Default|GetLastSquadNum))
  (Variables|Default|SetMemberNumber 1)
  (if (== 0 (Variables|Default|GetNumSquads))
    (if (not (== _lastsquadnum 0))
      (CallFunction|RandomSpawnPoint)
      (CallFunction|SpawnSingleSquad _lastsquadnum (Variables|Default|GetSpawnPoint)))
    (else
      (CallFunction|RandomSpawnPoint)
      (CallFunction|SpawnSingleSquad 5 (Variables|Default|GetSpawnPoint)))))

(fn RandomSpawnPoint
  (switch int (Math|Random|RandomInteger 5)
    (:0
      (Variables|Default|SetSpawnPoint (Variables|Default|GetSpawnPoint1)))
    (:1
      (Variables|Default|SetSpawnPoint (Variables|Default|GetSpawnPoint2)))
    (:2
      (Variables|Default|SetSpawnPoint (Variables|Default|GetSpawnPoint3)))
    (:3
      (Variables|Default|SetSpawnPoint (Variables|Default|GetSpawnPoint4)))
    (:4
      (Variables|Default|SetSpawnPoint (Variables|Default|GetSpawnPoint5)))))

(fn SpawnSingleSquad
  (params (SquadSize :type Integer :default 0) (SpawnPoint :type My%20Target%20Point%20Object%20Reference))
  (for _index (range 1 SquadSize)
    (AI|SpawnAIFromClass "/Game/Blueprints/AI/ProjectAngelisAI/AIGuard/AngelisEnemy2.AngelisEnemy2_C" "/Game/Blueprints/AI/ProjectAngelisAI/ProjectAngelisBT.ProjectAngelisBT" (Transformation|GetActorLocation SpawnPoint) (Transformation|GetActorRotation SpawnPoint) false)))