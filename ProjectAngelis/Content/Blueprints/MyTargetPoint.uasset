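; MyTargetPoint is an enemy spawn point that creates AngelisEnemy AI running ZombieBehaviorTree at its own transform.
; SpawnEnemy sets itself as the enemy's OwningSpawner, while SpawnSingleSquad spawns a given count in one loop without that link.
; It stores parent and two-child references and exposes a wrapper firing the Letsspawnenemy dispatcher.
; Its events are empty, and the delayed squad spawn is unfinished, with its logic disconnected.
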(event EventBeginPlay)

(event EventActorBeginOverlap
  (params (OtherActor :type Actor%20Object%20Reference)))

(event EventTick
  (params (DeltaSeconds :type Float%20%28single-precision%29)))

(fn ConstructionScript)

(fn Print
  (Development|PrintString "Hi"))

(fn CallSpawnEnemyDispatcher
  (Default|CallLetsspawnenemy))

(fn SpawnEnemy
  (bind _self self)
  (bind _returnvalue (AI|SpawnAIFromClass "/Game/Blueprints/AI/ProjectAngelisAI/AIGuard/AngelisEnemy.AngelisEnemy_C" "/Game/Blueprints/AI/Zombie/ZombieBehaviorTree.ZombieBehaviorTree" (Transformation|GetActorLocation _self) (Transformation|GetActorRotation _self) false))
  (bind _asangelis_enemy (Utilities|Casting|CastToAngelisEnemy _returnvalue))
  (Variables|/Game/Blueprints/AI/ProjectAngelisAI/AIGuard/AngelisEnemy.AngelisEnemy_C|SetOwning%20Spawner _asangelis_enemy self))

(fn SetChildren
  (params (InputChild1 :type My%20Target%20Point%20Object%20Reference) (InputChild2 :type My%20Target%20Point%20Object%20Reference))
  (Variables|Default|SetChild1 InputChild1)
  (Variables|Default|SetChild2 InputChild2))

(fn SetParent
  (params (InputParent :type Spawn%20Parent%20Object%20Reference))
  (Variables|Default|SetParent InputParent))

(fn SpawnSingleSquad
  (params (NumEnemies :type Integer))
  (bind _self self)
  (for _index (range 1 NumEnemies)
    (AI|SpawnAIFromClass "/Game/Blueprints/AI/ProjectAngelisAI/AIGuard/AngelisEnemy.AngelisEnemy_C" "/Game/Blueprints/AI/Zombie/ZombieBehaviorTree.ZombieBehaviorTree" (Transformation|GetActorLocation _self) (Transformation|GetActorRotation _self) false)))

(fn SpawnSingleSquadwithDelay)