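; Spawn_Friendly is an overlap trigger that works as an on/off button, broadcasting whether something has entered or left it.
; Begin and end overlap set the Intrigger1 flag and share one branch, which calls the Buttontrue1 or Buttonfalse1 event dispatcher.
; Each overlap event also toggles the collision component's visibility.
; No spawning logic lives in this Blueprint, despite its name.
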(event EventActorBeginOverlap
  (params (OtherActor :type Actor%20Object%20Reference))
  (Variables|Default|Setintrigger1 true)
  (if (Variables|Default|Getintrigger1)
    (Rendering|ToggleVisibility (Variables|Default|GetCollisionComponent) false)
    (Default|CallButtontrue1)
    (else
      (Rendering|ToggleVisibility (Variables|Default|GetCollisionComponent) false)
      (Default|CallButtonfalse1))))

(event EventActorEndOverlap
  (params (OtherActor :type Actor%20Object%20Reference))
  (Variables|Default|Setintrigger1 false)
  (if (Variables|Default|Getintrigger1)
    (Rendering|ToggleVisibility (Variables|Default|GetCollisionComponent) false)
    (Default|CallButtontrue1)
    (else
      (Rendering|ToggleVisibility (Variables|Default|GetCollisionComponent) false)
      (Default|CallButtonfalse1))))

(fn ConstructionScript)