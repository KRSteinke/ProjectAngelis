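; VR game mode that runs enemy waves, spawning AngelisEnemy2 pawns on a zombie behavior tree.
; InitWave advances the wave, randomizes two ambient sounds, splits per-wave counts into squads of five plus a remainder, and starts a looping timer.
; Each tick of that timer spawns a squad at one of five random points.
; Medium and heavy shares are computed but unused in spawning, and the squad count never decrements here.
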(event EventBeginPlay)

(event EventTick
  (params (DeltaSeconds :type Float%20%28single-precision%29)))

(fn ConstructionScript)

(fn SpawnEnemy
  (bind _spawnpoint1 (Variables|Default|GetSpawnPoint1))
  (AI|SpawnAIFromClass "/Game/Blueprints/AI/ProjectAngelisAI/AIGuard/AngelisEnemy2.AngelisEnemy2_C" "/Game/Blueprints/AI/Zombie/ZombieBehaviorTree.ZombieBehaviorTree" (Transformation|GetActorLocation _spawnpoint1) (Transformation|GetActorRotation _spawnpoint1) false))

(fn InitWave
  (bind _numsquads (Variables|Default|GetNumSquads))
  (bind _returnvalue (+ _numsquads 1))
  (Default|SetRandomAmbientSound (Variables|Default|GetAmbientSound1))
  (Default|SetRandomAmbientSound (Variables|Default|GetAmbientSound2))
  (Variables|Default|SetSquadNum 0)
  (bind _output_get (Variables|Default|SetWaveNumber (+ (Variables|Default|GetWaveNumber) 1)))
  (Variables|Default|SetCurrentEnemies (Utilities|Array|Get(acopy) (Variables|Default|GetEnemyNum) _output_get))
  (CallFunction|FindNumSquads)
  (if (== (Variables|Default|GetLastSquadNum) 0)
    (CallFunction|FindNumMeds _numsquads)
    ;[1 1 1] Find Num Heavies
    (CallFunction|FindNumHeavy _numsquads)
    (else
      ;[1 1 1] Find Num Meds
      (CallFunction|FindNumMeds _returnvalue)
      ;[1 1 1] Find Num Heavies
      (CallFunction|FindNumHeavy _returnvalue)))
  (Utilities|Time|SetTimerbyFunctionName self "SpawnSquadFromEnemy" 2e+01 true))

(fn FindNumMeds
  (params (NumSquads :type Integer :default 0))
  (bind _wavenumber (Variables|Default|GetWaveNumber))
  (bind _medenemies (Variables|Default|GetMedEnemies))
  (bind _item (Utilities|Array|Get(acopy) _medenemies _wavenumber))
  (bind _returnvalue (/ _item NumSquads))
  (bind _returnvalue_2 (Math|Integer|%(Integer) _item NumSquads))
  (Variables|Default|SetMedsPerSquad _returnvalue)
  (Development|PrintString (Utilities|String|Append "Num med is:" (Utilities|String|ToString(Integer) _returnvalue)))
  (Variables|Default|SetMedSpares _returnvalue_2)
  (Development|PrintString (Utilities|String|Append "Med spares are: " (Utilities|String|ToString(Integer) _returnvalue_2))))

(fn FindNumSquads
  (bind _enemynum (Variables|Default|GetEnemyNum))
  (bind _wavenumber (Variables|Default|GetWaveNumber))
  (bind _item (Utilities|Array|Get(acopy) _enemynum _wavenumber))
  (bind _returnvalue (/ _item 5))
  (bind _returnvalue_2 (Math|Integer|%(Integer) _item 5))
  (Variables|Default|SetCurrentEnemies _item)
  (Development|PrintString (Utilities|String|Append "Num Squads is:" (Utilities|String|ToString(Integer) _returnvalue)))
  (Variables|Default|SetNumSquads _returnvalue)
  (Development|PrintString (Utilities|String|Append "Last Squad Num is:" (Utilities|String|ToString(Integer) _returnvalue_2)))
  (Variables|Default|SetLastSquadNum _returnvalue_2))

(fn FindNumHeavy
  (params (NumSquads :type Integer :default 0))
  (bind _wavenumber (Variables|Default|GetWaveNumber))
  (bind _heavyenemies (Variables|Default|GetHeavyEnemies))
  (bind _item (Utilities|Array|Get(acopy) _heavyenemies _wavenumber))
  (bind _returnvalue (/ _item NumSquads))
  (bind _returnvalue_2 (Math|Integer|%(Integer) _item NumSquads))
  (Variables|Default|SetHeavyPerSquad _returnvalue)
  (Development|PrintString (Utilities|String|Append "Num med is:" (Utilities|String|ToString(Integer) _returnvalue)))
  (Variables|Default|SetHeavySpares _returnvalue_2)
  (Development|PrintString (Utilities|String|Append "Med spares are: " (Utilities|String|ToString(Integer) _returnvalue_2))))

(fn SpawnSquadfromEnemy
  (bind _lastsquadnum (Variables|Default|GetLastSquadNum))
  (Variables|Default|SetMemberNumber 1)
  (if (== 0 (Variables|Default|GetNumSquads))
    (if (not (== _lastsquadnum 0))
      (CallFunction|RandomSpawnPoint)
      (CallFunction|SpawnSingleSquad _lastsquadnum (Variables|Default|GetSpawnPoint)))
    (else
      (CallFunction|RandomSpawnPoint)
      (CallFunction|SpawnSingleSquad 5 (Variables|Default|GetSpawnPoint)))))

(fn RandomSpawnPoint
  (switch int (Math|Random|RandomInteger 5)
    (:0
      (Variables|Default|SetSpawnPoint (Variables|Default|GetSpawnPoint1)))
    (:1
      (Variables|Default|SetSpawnPoint (Variables|Default|GetSpawnPoint2)))
    (:2
      (Variables|Default|SetSpawnPoint (Variables|Default|GetSpawnPoint3)))
    (:3
      (Variables|Default|SetSpawnPoint (Variables|Default|GetSpawnPoint4)))
    (:4
      (Variables|Default|SetSpawnPoint (Variables|Default|GetSpawnPoint5)))))

(fn SpawnSingleSquad
  (params (SquadSize :type Integer :default 0) (SpawnPoint :type My%20Target%20Point%20Object%20Reference))
  (for _index (range 1 SquadSize)
    (Development|PrintString "Enemy Spawned")
    (AI|SpawnAIFromClass "/Game/Blueprints/AI/ProjectAngelisAI/AIGuard/AngelisEnemy2.AngelisEnemy2_C" "/Game/Blueprints/AI/Zombie/ZombieBehaviorTree.ZombieBehaviorTree" (Transformation|GetActorLocation SpawnPoint) (Transformation|GetActorRotation SpawnPoint) false)))