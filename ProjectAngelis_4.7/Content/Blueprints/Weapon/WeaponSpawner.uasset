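; Weapon spawner actor that periodically spawns a random weapon at its own transform.
; Tick increments WeaponDelta once per frame, then resets it and calls SpawnRandomWeapon on reaching WeaponThreshold, so timing is frame-rate dependent.
; SpawnRandomWeapon switches on a random integer across Proto and Dark variants of pistol, shotgun, assault rifle, sniper and rocket launcher.
; One of the eleven possible rolls has no case and spawns nothing.
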(event EventBeginPlay)

(event EventActorBeginOverlap
  (params (OtherActor :type Actor%20Object%20Reference)))

(event EventTick
  (params (DeltaSeconds :type Float%20%28single-precision%29))
  (bind _output_get (Variables|Default|SetWeaponDelta (+ 1 (Variables|Default|GetWeaponDelta))))
  (if (== _output_get (Variables|Default|GetWeaponThreshold))
    (Variables|Default|SetWeaponDelta 0)
    (CallFunction|SpawnRandomWeapon)))

(fn ConstructionScript)

(fn SpawnRandomWeapon
  (bind _self self)
  (bind _returnvalue (Transformation|GetActorTransform _self))
  (switch int (Math|Random|RandomInteger 11)
    (:0
      (Game|SpawnActorfromClass "/Game/Blueprints/Weapon/PistolProto.PistolProto_C" _returnvalue false 0))
    (:1
      (Game|SpawnActorfromClass "/Game/Blueprints/Weapon/PistolDark.PistolDark_C" _returnvalue false 0))
    (:2
      (Game|SpawnActorfromClass "/Game/Blueprints/Weapon/ShotgunProto.ShotgunProto_C" _returnvalue false 0))
    (:3
      (Game|SpawnActorfromClass "/Game/Blueprints/Weapon/ShotgunDark.ShotgunDark_C" _returnvalue false 0))
    (:4
      (Game|SpawnActorfromClass "/Game/Blueprints/Weapon/AssaultRifleProto.AssaultRifleProto_C" _returnvalue false 0))
    (:5
      (Game|SpawnActorfromClass "/Game/Blueprints/Weapon/AssaultRifleDark.AssaultRifleDark_C" _returnvalue false 0))
    (:6
      (Game|SpawnActorfromClass "/Game/Blueprints/Weapon/SniperProto.SniperProto_C" _returnvalue false 0))
    (:7
      (Game|SpawnActorfromClass "/Game/Blueprints/Weapon/SniperDark.SniperDark_C" _returnvalue false 0))
    (:8
      (Game|SpawnActorfromClass "/Game/Blueprints/Weapon/RocketLauncherProto.RocketLauncherProto_C" _returnvalue false 0))
    (:9
      (Game|SpawnActorfromClass "/Game/Blueprints/Weapon/RocketLauncherDark.RocketLauncherDark_C" _returnvalue false 0))))