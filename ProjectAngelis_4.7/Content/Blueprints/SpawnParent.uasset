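; SpawnParent is an enemy spawner that spawns one AngelisEnemy running ZombieBehaviorTree at its own transform on BeginPlay.
; It also stores two child references, which TestChildren tells to spawn enemies.
; Squad spawning is unfinished: FindNumSquads always computes from zero because its JustWaveNumbers wave lookup is disconnected, and the SpawnSingleSquad function looped by SpawnSquads is empty.
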(event EventBeginPlay
  (bind _self self)
  (bind _returnvalue (AI|SpawnAIFromClass "/Game/Blueprints/AI/ProjectAngelisAI/AIGuard/AngelisEnemy.AngelisEnemy_C" "/Game/Blueprints/AI/Zombie/ZombieBehaviorTree.ZombieBehaviorTree" (Transformation|GetActorLocation _self) (Transformation|GetActorRotation _self) false))
  (Utilities|Casting|CastToAngelisEnemy _returnvalue))

(event EventActorBeginOverlap
  (params (OtherActor :type Actor%20Object%20Reference)))

(event EventTick
  (params (DeltaSeconds :type Float%20%28single-precision%29)))

(fn ConstructionScript)

(fn SetChildren
  (params (InputChild1 :type My%20Target%20Point%20Object%20Reference) (InputChild2 :type My%20Target%20Point%20Object%20Reference))
  (Variables|Default|SetChild1 InputChild1)
  (Variables|Default|SetChild2 InputChild2))

(fn TestChildren
  (Default|SpawnEnemy (Variables|Default|GetChild1))
  (Default|SpawnEnemy (Variables|Default|GetChild2)))

(fn FindNumSquads
  (bind _returnvalue (Math|Conversions|ToFloat(Integer) 0))
  (bind _returnvalue_2 (/ _returnvalue 5.0))
  (bind _returnvalue_3 (Math|Float|Ceil _returnvalue_2))
  (bind _aswave_mode_bp (Utilities|Casting|CastToWaveMode_BP (Game|GetGameMode)))
  (Development|PrintString (Utilities|String|Append "Num Sqads is:" (Utilities|String|ToString(Integer) _returnvalue_3)))
  (Variables|Default|SetNumSquads _returnvalue_3))

(fn SpawnSquads
  (params (NumSquads :type Integer :default 0))
  (for _index (range 0 NumSquads)
    (CallFunction|SpawnSingleSquad)))

(fn SpawnSingleSquad)