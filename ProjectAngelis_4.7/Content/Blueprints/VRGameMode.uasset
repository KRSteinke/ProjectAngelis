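; VR game mode that runs wave-based enemy spawning from per-wave enemy count arrays.
; InitWave advances the wave, splits its total into squads of five plus a remainder, and starts a looping timer that spawns squads at four random spawn points.
; Once all squads are out and CurrentEnemies reaches zero, the next wave begins.
; Medium and heavy per-squad shares are calculated, but spawning uses only AngelisEnemy2 with ZombieBehaviorTree.
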(fn ConstructionScript)

(fn FindNumMeds
  (params (NumSquads :type Integer))
  (bind _wavenumber (Variables|Default|GetWaveNumber))
  (bind _medenemies (Variables|Default|GetMedEnemies))
  (bind _item (Utilities|Array|Get(acopy) _medenemies _wavenumber))
  (bind _returnvalue (/ _item NumSquads))
  (bind _returnvalue_2 (Math|Integer|%(Integer) _item NumSquads))
  (Variables|SquadComp|SetMedsPerSquad _returnvalue)
  (Development|PrintString (Utilities|String|Append "Num med is:" (Utilities|String|ToString(Integer) _returnvalue)))
  (Variables|SquadComp|SetMedSpares _returnvalue_2)
  (Development|PrintString (Utilities|String|Append "Med spares are: " (Utilities|String|ToString(Integer) _returnvalue_2))))

(fn SpawnSingleSquad
  (params (SquadSize :type Integer) (SpawnPoint :type My%20Target%20Point%20Object%20Reference))
  (Development|PrintString "In Spawn Single Squad")
  (for _index (range 1 SquadSize)
    (AI|SpawnAIFromClass "/Game/Blueprints/AI/ProjectAngelisAI/AIGuard/AngelisEnemy2.AngelisEnemy2_C" "/Game/Blueprints/AI/Zombie/ZombieBehaviorTree.ZombieBehaviorTree" (Transformation|GetActorLocation SpawnPoint) (Transformation|GetActorRotation SpawnPoint) false)))

(fn SpawnSquadfromEnemy
  (if (== 0 (Variables|Default|GetNumSquads))
    (if (== (Variables|Default|GetLastSquadNum) 0)
      (if (== (Variables|Default|GetCurrentEnemies) 0)
        (CallFunction|InitWave))
      (else
        (Utilities|RandomSpawnPoint
          (:Output
            (CallFunction|SpawnSingleSquad (Variables|Default|GetLastSquadNum) (Variables|Default|GetSpawnPoint))
            (Variables|Default|SetLastSquadNum 0)))))
    (else
      (Variables|Default|SetNumSquads (- (Variables|Default|GetNumSquads) 1))
      (Utilities|RandomSpawnPoint
        (:Output
          (CallFunction|SpawnSingleSquad 5 (Variables|Default|GetSpawnPoint)))))))

(fn InitWave
  (bind _numsquads (Variables|Default|GetNumSquads))
  (bind _returnvalue (+ _numsquads 1))
  (Variables|Default|SetSquadNum 0)
  (Variables|Default|SetWaveNumber (+ (Variables|Default|GetWaveNumber) 1))
  (CallFunction|FindNumSquads)
  (if (== (Variables|Default|GetLastSquadNum) 0)
    (CallFunction|FindNumMeds _numsquads)
    (CallFunction|FindNumHeavy _numsquads)
    (else
      (CallFunction|FindNumMeds _returnvalue)
      (CallFunction|FindNumHeavy _returnvalue)))
  (Utilities|Time|SetTimerbyFunctionName self "SpawnSquadFromEnemy" 2e+01 true))

(fn FindNumSquads
  (bind _enemynum (Variables|Default|GetEnemyNum))
  (bind _wavenumber (Variables|Default|GetWaveNumber))
  (bind _item (Utilities|Array|Get(acopy) _enemynum _wavenumber))
  (bind _returnvalue (/ _item 5))
  (bind _returnvalue_2 (Math|Integer|%(Integer) _item 5))
  (Variables|Default|SetCurrentEnemies _item)
  (Development|PrintString (Utilities|String|Append "Num Squads is:" (Utilities|String|ToString(Integer) _returnvalue)))
  (Variables|Default|SetNumSquads _returnvalue)
  (Development|PrintString (Utilities|String|Append "Last Squad Num is:" (Utilities|String|ToString(Integer) _returnvalue_2)))
  (Variables|Default|SetLastSquadNum _returnvalue_2))

(fn FindNumHeavy
  (params (NumSquads :type Integer))
  (bind _wavenumber (Variables|Default|GetWaveNumber))
  (bind _heavyenemies (Variables|Default|GetHeavyEnemies))
  (bind _item (Utilities|Array|Get(acopy) _heavyenemies _wavenumber))
  (bind _returnvalue (/ _item NumSquads))
  (bind _returnvalue_2 (Math|Integer|%(Integer) _item NumSquads))
  (Variables|SquadComp|SetHeavyPerSquad _returnvalue)
  (Development|PrintString (Utilities|String|Append "Num Heavy is:" (Utilities|String|ToString(Integer) _returnvalue)))
  (Variables|SquadComp|SetHeavySpares _returnvalue_2)
  (Development|PrintString (Utilities|String|Append "Heavy spares are: " (Utilities|String|ToString(Integer) _returnvalue_2))))