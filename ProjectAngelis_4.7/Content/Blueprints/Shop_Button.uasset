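; Shop button trigger actor that shows a text prompt and signals whether something is standing in it.
; Begin and end overlap, unfiltered by actor, set an in-trigger flag and share one branch that calls the ButtonTrue or ButtonFalse dispatcher for listeners.
; The same branch uses ToggleVisibility on the TextRender, so each overlap event flips the text rather than setting it explicitly.
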(event EventBeginPlay)

(event EventActorBeginOverlap
  (params (OtherActor :type Actor%20Object%20Reference))
  (Variables|Default|Setintrigger true)
  (if (Variables|Default|Getintrigger)
    (Rendering|ToggleVisibility (Variables|Default|GetTextRender) true)
    (Default|CallButtonTrue)
    (else
      (Rendering|ToggleVisibility (Variables|Default|GetTextRender) false)
      (Default|CallButtonFalse))))

(event EventTick
  (params (DeltaSeconds :type Float%20%28single-precision%29)))

(event EventActorEndOverlap
  (params (OtherActor :type Actor%20Object%20Reference))
  (Variables|Default|Setintrigger false)
  (if (Variables|Default|Getintrigger)
    (Rendering|ToggleVisibility (Variables|Default|GetTextRender) true)
    (Default|CallButtonTrue)
    (else
      (Rendering|ToggleVisibility (Variables|Default|GetTextRender) false)
      (Default|CallButtonFalse))))

(fn ConstructionScript)