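; Ambient sound actor that starts a dark atmospheric track when play begins.
; BeginPlay always plays the Dark_Heavy_Sad sound at the world origin.
; A separate SetRandomAmbientSound function picks one of eighteen mood tracks at random and plays it at the origin, but nothing in this Blueprint calls it.
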(event EventBeginPlay
  (Audio|PlaySoundatLocation "/Game/SMAtmospheres/Wavs/Dark_Heavy_Sad.Dark_Heavy_Sad" "0, 0, 0"))

(event EventTick
  (params (DeltaSeconds :type Float%20%28single-precision%29)))

(fn ConstructionScript)

(fn SetRandomAmbientSound
  (switch int (Math|Random|RandomInteger 18)
    (:0
      (Audio|PlaySoundatLocation "/Game/SMAtmospheres/Wavs/Dark_Heavy_Sad.Dark_Heavy_Sad" "0, 0, 0"))
    (:1
      (Audio|PlaySoundatLocation "/Game/SMAtmospheres/Wavs/Dark_Subtle_Atmosphere.Dark_Subtle_Atmosphere" "0, 0, 0"))
    (:2
      (Audio|PlaySoundatLocation "/Game/SMAtmospheres/Wavs/General_Dark_Room.General_Dark_Room" "0, 0, 0"))
    (:3
      (Audio|PlaySoundatLocation "/Game/SMAtmospheres/Wavs/High_Anxiety.High_Anxiety" "0, 0, 0"))
    (:4
      (Audio|PlaySoundatLocation "/Game/SMAtmospheres/Wavs/Low_Dark_Very_Subtle.Low_Dark_Very_Subtle" "0, 0, 0"))
    (:5
      (Audio|PlaySoundatLocation "/Game/SMAtmospheres/Wavs/Low_Darkness.Low_Darkness" "0, 0, 0"))
    (:6
      (Audio|PlaySoundatLocation "/Game/SMAtmospheres/Wavs/Low_Rumble.Low_Rumble" "0, 0, 0"))
    (:7
      (Audio|PlaySoundatLocation "/Game/SMAtmospheres/Wavs/Magical_Realization.Magical_Realization" "0, 0, 0"))
    (:8
      (Audio|PlaySoundatLocation "/Game/SMAtmospheres/Wavs/MediumTense_Atmosphere.MediumTense_Atmosphere" "0, 0, 0"))
    (:9
      (Audio|PlaySoundatLocation "/Game/SMAtmospheres/Wavs/Neutral_Amosphere.Neutral_Amosphere" "0, 0, 0"))
    (:10
      (Audio|PlaySoundatLocation "/Game/SMAtmospheres/Wavs/Neutral_Dark_Quick.Neutral_Dark_Quick" "0, 0, 0"))
    (:11
      (Audio|PlaySoundatLocation "/Game/SMAtmospheres/Wavs/Neutral_Magical_Quick.Neutral_Magical_Quick" "0, 0, 0"))
    (:12
      (Audio|PlaySoundatLocation "/Game/SMAtmospheres/Wavs/Neutral_Tense_Quick.Neutral_Tense_Quick" "0, 0, 0"))
    (:13
      (Audio|PlaySoundatLocation "/Game/SMAtmospheres/Wavs/Subtle_Slightly_Magical.Subtle_Slightly_Magical" "0, 0, 0"))
    (:14
      (Audio|PlaySoundatLocation "/Game/SMAtmospheres/Wavs/Swirling_Atmosphere.Swirling_Atmosphere" "0, 0, 0"))
    (:15
      (Audio|PlaySoundatLocation "/Game/SMAtmospheres/Wavs/Swirling_Bridge.Swirling_Bridge" "0, 0, 0"))
    (:16
      (Audio|PlaySoundatLocation "/Game/SMAtmospheres/Wavs/Tense_Subtle.Tense_Subtle" "0, 0, 0"))
    (:17
      (Audio|PlaySoundatLocation "/Game/SMAtmospheres/Wavs/Tense_Subtle_Slightly_Magical.Tense_Subtle_Slightly_Magical" "0, 0, 0"))))