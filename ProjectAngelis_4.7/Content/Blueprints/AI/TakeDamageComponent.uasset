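; Actor component that tracks health and handles death for the player and AngelisEnemy2 AI.
; It binds to the owner's any-damage event and subtracts damage unless dead or invulnerable.
; At zero health players are destroyed immediately; enemies stop AI, play a random death animation, ragdoll, then are removed with their weapon after a delay.
; Tick-counted health regeneration logic is present but disconnected.
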(event Custom|CustomEvent_1
  (params (Damage :type Float%20%28single-precision%29 :default 0.0) (DamageType :type Damage%20Type%20Object%20Reference) (InstigatedBy :type Controller%20Object%20Reference) (DamageCauser :type Actor%20Object%20Reference))
  (CallFunction|UpdateHealth Damage)
  (Variables|Default|SetRecentlyTookDamage true)
  (Variables|Default|SetTookDamageTick 0))

(event Custom|UpdateHealth
  (params (Damage :type Float%20%28single-precision%29 :default 0.0))
  (if (not (Variables|Default|GetIsDead))
    (if (not (Variables|Default|GetInvulnerable))
      (Variables|Default|SetHealth (- (Variables|Default|GetHealth) Damage))
      (CallFunction|CheckforDeath))))

(event Custom|CheckForDeath
  (bind _returnvalue (Components|GetOwner))
  (if (<= (Variables|Default|GetHealth) 0.0)
    (Variables|Default|SetIsDead true)
    (Utilities|IsValid _returnvalue
      (:Is%20Valid
        (if (Variables|Default|GetIsPlayer)
          (Actor|DestroyActor _returnvalue)
          (else
            (bind _returnvalue_2 (AI|GetAIController _returnvalue))
            (bind _asangelis_enemy_2 (Utilities|Casting|CastToAngelisEnemy2 (Pawn|GetControlledPawn _returnvalue_2)))
            (Default|SetDead _asangelis_enemy_2)
            (AI|Logic|StopLogic _returnvalue_2 "")
            (Components|DestroyComponent _returnvalue_2)
            (Components|DestroyComponent (Variables|/Script/ProjectAngelis.AngelisCharacter|GetCollisionComp _asangelis_enemy_2) _asangelis_enemy_2)
            (Components|Animation|PlayAnimation (Variables|/Script/Engine.Character|GetMesh _asangelis_enemy_2) (Utilities|Select :Index (Math|Random|RandomIntegerinRange 0 2) :Option%200 "/Game/ProtoCharacters/Death_1_Prototype.Death_1_Prototype" :Option%201 "/Game/ProtoCharacters/Death_2_Prototype.Death_2_Prototype" :Option%202 "/Game/ProtoCharacters/Death_3_Prototype.Death_3_Prototype") false)
            (Utilities|FlowControl|Delay 0.2)
            (Physics|SetSimulatePhysics (Variables|/Script/Engine.Character|GetMesh _asangelis_enemy_2) true)
            (Utilities|FlowControl|Delay 1e+01)
            (bind _returnvalue_3 (Class|AngelisCharacter|GetCurrentWeapon _asangelis_enemy_2))
            (Actor|DestroyActor _returnvalue_3)
            (Actor|DestroyActor _returnvalue)))))))

(event EventInitializeComponent
  (EventDispatchers|BindEventtoOnTakeAnyDamage (Components|GetOwner) (delegate Custom|CustomEvent_1)))

(fn ChangeHealth
  (params (HealthDelta :type Float%20%28single-precision%29 :default 0.0))
  (Variables|Default|SetHealth (+ HealthDelta (Variables|Default|GetHealth))))