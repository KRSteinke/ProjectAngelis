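; Wave-based game mode that tracks enemy deaths and spawns AI enemy squads for each wave.
; When the wave's count hits zero, EnemyDied advances the wave, splits its total into five-enemy squads plus a remainder, and spawns one squad.
; SpawnSingleSquad ignores its spawn point input, picking one of four at random, and makes the fifth member a leader with its own behavior tree.
; Medium-enemy splits are computed but unused in spawning.
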(event EventBeginPlay)

(event EventTick
  (params (DeltaSeconds :type Float%20%28single-precision%29)))

(fn ConstructionScript)

(fn EnemyDied
  (bind _currentnumenemies (CallFunction|DecrementEnemies))
  (Development|PrintString (Utilities|String|Append "Current Enemies: " (Utilities|String|ToString(Integer) _currentnumenemies)))
  (if (== _currentnumenemies 0)
    (CallFunction|InitWave)
    (CallFunction|SpawnSquadfromEnemy)))

(fn SetSpawnPoint
  (params (LevelSpawnPoint :type My%20Target%20Point%20Object%20Reference))
  (bind _output_get (Variables|Default|SetSpawnPoint1 LevelSpawnPoint))
  (AI|SpawnAIFromClass "/Game/Blueprints/AI/ProjectAngelisAI/AIGuard/AngelisEnemy.AngelisEnemy_C" "/Game/Blueprints/AI/Zombie/ZombieBehaviorTree.ZombieBehaviorTree" (Transformation|GetActorLocation _output_get) (Transformation|GetActorRotation _output_get) false))

(fn IncrementLevel
  (bind _output_get (Variables|Default|SetWave%20Number (+ 1 (Variables|Default|GetWave%20Number))))
  (Development|PrintString (Utilities|String|Append "current level after increment:" (Utilities|String|ToString(Integer) _output_get))))

(fn DecrementEnemies
  (bind _enemynumber (Variables|Default|GetEnemyNumber))
  (bind _wave_number (Variables|Default|GetWave%20Number))
  (bind _item (Utilities|Array|Get(acopy) _enemynumber _wave_number))
  (Utilities|Array|SetArrayElem _enemynumber _wave_number (- _item 1))
  (return _item))

(fn SpawnEnemies
  (params (SpawnPoint :type My%20Target%20Point%20Object%20Reference) (NumEnemies :type Integer :default 0))
  (for _index (range 0 NumEnemies)
    (AI|SpawnAIFromClass "/Game/Blueprints/AI/ProjectAngelisAI/AIGuard/AngelisEnemy.AngelisEnemy_C" "/Game/Blueprints/AI/Zombie/ZombieBehaviorTree.ZombieBehaviorTree" (Transformation|GetActorLocation SpawnPoint) (Transformation|GetActorRotation SpawnPoint) false)))

(fn TestPrint
  (Development|PrintString "Game Mode"))

(fn TestSpawn
  (bind _spawnpoint1 (Variables|Default|GetSpawnPoint1))
  (AI|SpawnAIFromClass "/Game/Blueprints/AI/ProjectAngelisAI/AIGuard/AngelisEnemy.AngelisEnemy_C" "/Game/Blueprints/AI/Zombie/ZombieBehaviorTree.ZombieBehaviorTree" (Transformation|GetActorLocation _spawnpoint1) (Transformation|GetActorRotation _spawnpoint1) false))

(fn FindNumMeds
  (params (NumSquads :type Integer))
  (bind _medenemies (Variables|Default|GetMedEnemies))
  (bind _wave_number (Variables|Default|GetWave%20Number))
  (bind _item (Utilities|Array|Get(acopy) _medenemies _wave_number))
  (bind _returnvalue (/ _item NumSquads))
  (bind _returnvalue_2 (Math|Integer|%(Integer) _item NumSquads))
  (Variables|SquadComp|SetMedPerSquad _returnvalue)
  (Development|PrintString (Utilities|String|Append "Num Med is: " (Utilities|String|ToString(Integer) _returnvalue)))
  (Variables|SquadComp|SetMedSpares _returnvalue_2)
  (Development|PrintString (Utilities|String|Append "Med Spares Are:" (Utilities|String|ToString(Integer) _returnvalue_2))))

(fn SpawnSingleSquad
  (params (SpawnPoint :type My%20Target%20Point%20Object%20Reference) (SpawnNumber :type Integer :default 0))
  (bind _spawnpoint (Utilities|RandomSpawnPoint)
    (:Output
      (for _index (range 1 SpawnNumber)
        (if (== _index 5)
          (AI|SpawnAIFromClass "/Game/Blueprints/AI/ProjectAngelisAI/AIGuard/AngelisEnemyLeader.AngelisEnemyLeader_C" "/Game/Blueprints/AI/ProjectAngelisAI/ProjectAngelisBT.ProjectAngelisBT" (Transformation|GetActorLocation _spawnpoint) (Transformation|GetActorRotation _spawnpoint) false)
          (Development|PrintString "Spawned Leader")
          (else
            (AI|SpawnAIFromClass "/Game/Blueprints/AI/ProjectAngelisAI/AIGuard/AngelisEnemy2.AngelisEnemy2_C" "/Game/Blueprints/AI/Zombie/ZombieBehaviorTree.ZombieBehaviorTree" (Transformation|GetActorLocation _spawnpoint) (Transformation|GetActorRotation _spawnpoint) false)
            (Development|PrintString "Spawned Follower")))))))

(fn SpawnSquads
  (params (SquadNum :type Integer :default 0) (LastSquadNum :type Integer :default 0))
  (Variables|Default|SetTempSquadNum SquadNum)
  (Variables|Default|SetLastSquadNum LastSquadNum)
  (while (> (Variables|Default|GetTempSquadNum) 0)
    (switch int (Variables|Default|GetNextSpawnPoint)
      (:Default
        (Development|PrintString "Error in Spawn Squads While Loop")
        (Variables|Default|SetTempSquadNum 0))
      (:0
        (CallFunction|SpawnSingleSquad (Variables|Default|GetSpawnPoint1) 5)
        (Variables|Default|SetNextSpawnPoint (+ 1 (Variables|Default|GetNextSpawnPoint)) :!label _label)
        (Variables|Default|SetTempSquadNum (- (Variables|Default|GetTempSquadNum) 1) :!label _label_2))
      (:1
        (CallFunction|SpawnSingleSquad (Variables|Default|GetSpawnPoint2) 5)
        (goto _label))
      (:2
        (CallFunction|SpawnSingleSquad (Variables|Default|GetSpawnPoint3) 5)
        (goto _label))
      (:3
        (CallFunction|SpawnSingleSquad (Variables|Default|GetSpawnPoint4) 5)
        (Variables|Default|SetNextSpawnPoint 0)
        (goto _label_2))))
  (Development|PrintString "While Loop Completed")
  (switch int (Variables|Default|GetNextSpawnPoint)
    (:Default
      (Development|PrintString "Error in last squad"))
    (:0
      (CallFunction|SpawnSingleSquad (Variables|Default|GetSpawnPoint1) (Variables|Default|GetLastSquadNum)))
    (:1
      (CallFunction|SpawnSingleSquad (Variables|Default|GetSpawnPoint2) (Variables|Default|GetLastSquadNum)))
    (:2
      (CallFunction|SpawnSingleSquad (Variables|Default|GetSpawnPoint3) (Variables|Default|GetLastSquadNum)))
    (:3
      (CallFunction|SpawnSingleSquad (Variables|Default|GetSpawnPoint4) (Variables|Default|GetLastSquadNum)))))

(fn SpawnSquadfromEnemy
  (if (== 0 (Variables|Default|GetNumSquads))
    (Variables|Default|SetNumSquads (- (Variables|Default|GetNumSquads) 1))
    (bind _spawnpoint (Utilities|RandomSpawnPoint)
      (:Output
        (CallFunction|SpawnSingleSquad _spawnpoint (Variables|Default|GetLastSquadNum))))
    (else
      (Variables|Default|SetNumSquads (- (Variables|Default|GetNumSquads) 1))
      (bind _spawnpoint_2 (Utilities|RandomSpawnPoint)
        (:Output
          (CallFunction|SpawnSingleSquad _spawnpoint_2 5))))))

(fn InitWave
  (Variables|Default|SetWave%20Number (+ (Variables|Default|GetWave%20Number) 1))
  (bind (_numsquads _lastsquadnum) (CallFunction|FindNumSquads))
  (if (== _lastsquadnum 0)
    (CallFunction|FindNumMeds _numsquads)
    (else
      (CallFunction|FindNumMeds (+ _numsquads 1))))
  (Variables|Default|SetNumSquads _numsquads)
  (Variables|Default|SetLastSquadNum _lastsquadnum))

(fn FindNumSquads
  (bind _wave_number (Variables|Default|GetWave%20Number))
  (bind _enemynumber (Variables|Default|GetEnemyNumber))
  (bind _item (Utilities|Array|Get(acopy) _enemynumber _wave_number))
  (bind _returnvalue (/ _item 5))
  (bind _returnvalue_2 (Math|Integer|%(Integer) _item 5))
  (Variables|Default|SetCurrentEnemies _item)
  (Development|PrintString (Utilities|String|Append "Num Squads is: " (Utilities|String|ToString(Integer) _returnvalue)))
  (Development|PrintString (Utilities|String|Append "Last Squad Num " (Utilities|String|ToString(Integer) _returnvalue_2)))
  (return _returnvalue _returnvalue_2))

(fn FindNumHeavy
  (params (NumSquads :type Integer))
  (bind _heavyenemies (Variables|Default|GetHeavyEnemies))
  (bind _wave_number (Variables|Default|GetWave%20Number))
  (bind _item (Utilities|Array|Get(acopy) _heavyenemies _wave_number))
  (bind _returnvalue (/ _item NumSquads))
  (bind _returnvalue_2 (Math|Integer|%(Integer) _item NumSquads))
  (Variables|SquadComp|SetMedPerSquad _returnvalue)
  (Development|PrintString (Utilities|String|Append "Num Heavy is: " (Utilities|String|ToString(Integer) _returnvalue)))
  (Variables|SquadComp|SetMedSpares _returnvalue_2)
  (Development|PrintString (Utilities|String|Append "Heavy Spares Are:" (Utilities|String|ToString(Integer) _returnvalue_2))))